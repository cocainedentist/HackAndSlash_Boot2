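; BP_SkillAroundActor is a skill actor that damages things around its instigator with an orbiting damage point.
; Each tick it snaps to the instigator's location and rotates its SpringArm a fixed step, independent of delta time.
; A fast looping timer applies radial damage at the Sphere's location, ignoring and crediting the instigator.
; Each damage pulse also draws a debug sphere showing the radius.
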(event EventBeginPlay
  (|CallParentFunction)
  (Utilities|Time|SetTimerbyFunctionName 0 "ApplyDamage" 0.05 true))

(event EventTick
  (params (DeltaSeconds :type Float%20%28single-precision%29))
  (Transformation|SetActorLocation (Transformation|GetActorLocation (Variables|Default|GetInstigator)) false false)
  (Transformation|AddRelativeRotation (Variables|Default|GetSpringArm) "0.000000,3.000000,0.000000" false false))

(fn ConstructionScript
  (|CallParentFunction))

(fn ApplyDamage
  (bind _instigator (Variables|Default|GetInstigator))
  (Rendering|Debug|DrawDebugSphere (Transformation|GetWorldLocation (Variables|Default|GetSphere)) (Variables|Default|GetRadius) 12 "(R=0.000000,G=1.000000,B=0.004107,A=1.000000)" 3.0 1.0)
  (Game|Damage|ApplyRadialDamage 2e+01 (Transformation|GetWorldLocation (Variables|Default|GetSphere)) (Variables|Default|GetRadius) 0 (Utilities|Array|MakeArray _instigator) self (Pawn|GetController _instigator) false "ECC_Visibility"))
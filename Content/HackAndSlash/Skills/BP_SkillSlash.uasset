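; BP_SkillSlash is a slash skill actor that deals repeated radial damage while attached to the Character that instigated it.
; On BeginPlay it attaches itself to that Character, sets its relative transform and starts a fast looping timer for ApplyDamage.
; Each tick of the timer applies radial damage around the Sphere component, ignoring and crediting the instigator, and draws a debug sphere at the same location.
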(event EventBeginPlay
  (|CallParentFunction)
  (bind _ascharacter (Utilities|Casting|CastToCharacter (Variables|Default|GetInstigator)))
  (Transformation|AttachActorToActor _ascharacter "None" "KeepRelative" "KeepRelative" "KeepRelative" true)
  (Transformation|SetActorRelativeTransform (Math|Transform|MakeTransform "0, 0, 0" "0, 0, 0" "1.000000,1.000000,1.000000") false false)
  (Utilities|Time|SetTimerbyFunctionName 0 "ApplyDamage" 0.05 true))

(fn ConstructionScript
  (|CallParentFunction))

(fn ApplyDamage
  (bind _instigator (Variables|Default|GetInstigator))
  (Rendering|Debug|DrawDebugSphere (Transformation|GetWorldLocation (Variables|Default|GetSphere)) (Variables|Default|GetRadius) 12 "(R=0.000000,G=0.036824,B=1.000000,A=1.000000)" 3.0 1.0)
  (Game|Damage|ApplyRadialDamage 2e+03 (Transformation|GetWorldLocation (Variables|Default|GetSphere)) (Variables|Default|GetRadius) 0 (Utilities|Array|MakeArray _instigator) self (Pawn|GetController _instigator) false "ECC_Visibility"))
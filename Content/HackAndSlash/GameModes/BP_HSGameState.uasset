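; Game state Blueprint for the hack-and-slash mode, holding the current game state enum and the time elapsed since the last change request.
; Tick accumulates delta seconds into that timer.
; ChangeGameState resets the timer on every call, then stores and broadcasts the new state through an event dispatcher only if it differs.
; A repeated state just prints a debug string.
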(event EventTick
  (params (DeltaSeconds :type Float%20%28single-precision%29))
  (Variables|Default|SetTotalDeltaSeconds (+ DeltaSeconds (Variables|Default|GetTotalDeltaSeconds))))

(fn ConstructionScript)

(fn ChangeGameState
  (params (GameState :type EN_GameState%20Enum :default "NewEnumerator0"))
  (Variables|Default|SetTotalDeltaSeconds 0.0)
  (if (Utilities|Enum|NotEqual(Enum) GameState (Variables|Default|GetGameState))
    (bind _output_get (Variables|Default|SetGameState GameState))
    (Default|CallEventDispatcherChangeGameState _output_get)
    (else
      (Development|PrintString "False!"))))
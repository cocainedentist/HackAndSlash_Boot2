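; BP_HSGameMode is the Hack and Slash game mode that drives match flow through BP_HSGameState.
; On BeginPlay it binds to the state-change dispatcher and switches straight to Play.
; The change handler uses game-only input with a hidden cursor for Ready and Play, and pauses with UI-only input and a cursor for End.
; Tick polls the Ready state and advances to Play after a five-second threshold.
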(event EventBeginPlay
  (bind _asbp_hsgame_state (Utilities|Casting|CastToBP_HSGameState (Game|GetGameState)))
  (EventDispatchers|BindEventtoEventDispatcherChangeGameState _asbp_hsgame_state (EventDispatchers|CreateEvent :!event EventChangeGameState))
  (Default|ChangeGameState _asbp_hsgame_state "NewEnumerator1"))

(event EventTick
  (params (DeltaSeconds :type Float%20%28single-precision%29))
  (bind _asbp_hsgame_state (Utilities|Casting|CastToBP_HSGameState (Game|GetGameState)))
  (switch Utilities|FlowControl|Switch|SwitchonEN_GameState (Variables|/Game/HackAndSlash/GameModes/BP_HSGameState.BP_HSGameState_C|GetGameState _asbp_hsgame_state)
    (:NewEnumerator0
      (CallFunction|UpdateReady _asbp_hsgame_state))))

(fn ConstructionScript)

(fn EventChangeGameState
  (params (GameState :type EN_GameState%20Enum :default "NewEnumerator0"))
  (bind _returnvalue (Game|GetPlayerController 0))
  (bind _returnvalue_2 (Game|GetPlayerController 0))
  (switch Utilities|FlowControl|Switch|SwitchonEN_GameState GameState
    (:NewEnumerator0
      (Input|SetInputModeGameOnly _returnvalue false :!label _label)
      (Variables|/Script/Engine.PlayerController|SetbShowMouseCursor _returnvalue false))
    (:NewEnumerator1
      (goto _label))
    (:NewEnumerator2
      (Game|SetGamePaused true)
      (Input|SetInputModeUIOnly _returnvalue_2 0 "DoNotLock" false)
      (Variables|/Script/Engine.PlayerController|SetbShowMouseCursor _returnvalue_2 true))))

(fn UpdateReady
  (params (InputPin :type BP%20HS%20Game%20State%20Object%20Reference))
  (if (>= (Variables|/Game/HackAndSlash/GameModes/BP_HSGameState.BP_HSGameState_C|GetTotalDeltaSeconds InputPin) 5.0)
    (Default|ChangeGameState InputPin "NewEnumerator1")
    (else
      (return InputPin))))